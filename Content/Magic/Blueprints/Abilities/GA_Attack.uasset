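; GA_Attack is a gameplay ability that performs a montage-driven attack and damages the target it hits.
; On activation it commits, plays the attack montage and waits once for a Character.Damaged gameplay event, applying GE_Damage to that event's target data.
; The ability ends when the montage completes, blends out or is interrupted, and OnEndAbility ends the stored wait task.
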(event Ability|EventActivateAbility
  (Ability|CommitAbility)
  (Animation|Montage|PlayMontage (.SkeletalMeshComponent (Utilities|Struct|BreakGameplayAbilityActorInfo (Ability|GetActorInfo))) "/Game/BattleWizardPolyart/Animations/AM_Attack02MaintainAnim.AM_Attack02MaintainAnim"
    (:then
      (bind (_asynctaskproxy _payload) (Ability|Tasks|WaitGameplayEvent "(TagName=\"Character.Damaged\")" 0 true)
        (:then
          (Variables|Default|SetWaitTask _asynctaskproxy))
        (:EventReceived
          (GameplayEffects|ApplyGameplayEffectToTarget (.TargetData (Utilities|Struct|BreakGameplayEventData _payload)) "/Game/Magic/Blueprints/Abilities/GE_Damage.GE_Damage_C" 1 1))))
    (:OnCompleted
      (Ability|EndAbility :!label _label))
    (:OnBlendOut
      (goto _label))
    (:OnInterrupted
      (goto _label))))

(event Ability|EventOnEndAbility
  (params (bWasCancelled :type Boolean))
  (bind _waittask (Variables|Default|GetWaitTask))
  (Utilities|IsValid _waittask
    (:Is%20Valid
      (GameplayTasks|EndTask _waittask))))